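; Graffiti generator actor that spells out a Word string as a row of decals, built entirely in the Construction Script.
; Each character's DT_Alphabet row supplies the atlas frame for a dynamic decal material, alongside font atlas, color and emissive.
; GetDecalOffset spaces letters by scaled atlas cell width plus Offset, leaving gaps for characters missing from the table.
; An optional billboard is raised above the averaged decal position.
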(event `self.ReceiveBeginPlay`)

(fn `GetDecalOffset`
  (params (Order :type Integer))
  (returns (Offset :type "Vector Structure"))
  (return (`KismetMathLibrary.MakeVector` (+ (.x (* (`self.Offset`) Order)) (* (* Order (/ (`Texture2D.Blueprint_GetSizeX` (`self.FontAtlas`)) (`self.AtlasColumnCount`))) (`self.Scale`))) (.y (* (`self.Offset`) Order)) (.z (* (`self.Offset`) Order)))))

(fn `UserConstructionScript`
  (locals (TotalWidth :type "Vector Structure"))
  (bind _scale (`self.Scale`))
  (bind _returnvalue (`KismetStringLibrary.GetCharacterArrayFromString` (`self.Word`)))
  (bind _returnvalue_2 (`KismetArrayLibrary.Array_Length` _returnvalue))
  (`SceneComponent.SetVisibility` (`self.Billboard`) (`self.ShowBilboard`) false)
  (for (_array_element _array_index) _returnvalue
    (bind _returnvalue_3 (`|GetDataTableRow` "/Game/LevelDesignToolKit/GrafittiSystem/Blueprints/DT_Alphabet.DT_Alphabet" (`KismetStringLibrary.Conv_StringToName` _array_element))
      (:`then`
        (bind _returnvalue_4 (`AddComponent|NODE_AddDecalComponent-0` :`RelativeTransform` (`KismetMathLibrary.MakeTransform` (select `bool` (== _array_index 0) :`false` (`self.GetDecalOffset` _array_index)) (`self.Rotation`) (`KismetMathLibrary.MakeVector` _scale _scale _scale))))
        (bind _returnvalue_5 (`DecalComponent.CreateDynamicMaterialInstance` _returnvalue_4))
        (`MaterialInstanceDynamic.SetScalarParameterValue` _returnvalue_5 "Frame" (`.ID_3_4E4685B34243746D2C403D9307431C7D` (break `/Game/LevelDesignToolKit/GrafittiSystem/Blueprints/SAlphabet` _returnvalue_3)))
        (`MaterialInstanceDynamic.SetScalarParameterValue` _returnvalue_5 "Power" (`self.Emissive`))
        (`MaterialInstanceDynamic.SetVectorParameterValue` _returnvalue_5 "Color" (`self.Color`))
        (`MaterialInstanceDynamic.SetTextureParameterValue` _returnvalue_5 "Atlas" (`self.FontAtlas`))
        (set `local.TotalWidth` (+ (`local.TotalWidth`) (`SceneComponent.RelativeLocation` _returnvalue_4))))))
  ;[1 1 1] Centered Bilboard
  (`SceneComponent.K2_SetRelativeLocation` (`self.Billboard`) (+ (/ (`local.TotalWidth`) (select `bool` (> _returnvalue_2 0) :`false` 1 :`true` _returnvalue_2)) (* (`SceneComponent.GetUpVector` (`self.Scene`)) 50.0)) false false))