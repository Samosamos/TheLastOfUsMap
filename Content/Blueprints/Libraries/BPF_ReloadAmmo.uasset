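; Blueprint function library holding ReloadAmmo, a stateless calculation for reloading a weapon magazine from reserve ammo.
; It compares the missing rounds, max minus loaded, against the ammo in stock.
; With enough stock it fills the magazine and deducts the difference; otherwise it moves all remaining stock into the magazine and zeroes the reserve.
; It returns both new counts to the caller.
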(fn `ReloadAmmo`
  (params (MaxLoadedAmmo :type Integer) (LoadedAmmo :type Integer) (AmmoInStock :type Integer))
  (returns (NewLoadedAmmo :type Integer) (NewAmmoInStock :type Integer))
  (bind _loadedammo (`local.LoadedAmmo`))
  (bind _returnvalue (- (`local.MaxLoadedAmmo`) _loadedammo))
  (if (>= (`local.AmmoInStock`) _returnvalue)
    (return (+ _loadedammo _returnvalue) (- (`local.AmmoInStock`) _returnvalue))
    (else
      (return (+ (`local.LoadedAmmo`) (`local.AmmoInStock`)) 0))))