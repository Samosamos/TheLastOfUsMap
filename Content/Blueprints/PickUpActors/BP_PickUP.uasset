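; BP_PickUP is a pickup actor that shows proximity and selection cues and can be collected by the player.
; Each tick it shows its Billboard within a distance threshold and rotates its Text to face the player camera.
; Blueprint interface calls toggle the Text on selection, report the pickup distance, and trigger pickup, which plays a sound and destroys the actor.
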(event `self.ReceiveBeginPlay`
  (`SceneComponent.SetVisibility` (`self.Text`) false true))

(event `self.ReceiveTick`
  (params (DeltaSeconds :type "Float (single-precision)"))
  (`SceneComponent.SetVisibility` (`self.Billboard`) (<= (`self.DistanceFromPlayer`) (`self.DistanceThreshold`)) true)
  (`self.RotateTowardsPlayer` (`self.Text`)))

(event `/Game/Blueprints/PickUpActors/BPI_PickUp.BPI ObjectIsSelected`
  (params (IsSelected :type Boolean))
  (`SceneComponent.SetVisibility` (`self.Text`) IsSelected true))

(event `/Game/Blueprints/PickUpActors/BPI_PickUp.BPI PickObject`
  (`self.PickObject`))

(fn `BPI GetPickUpDistance`
  (returns (Distance :type "Float (double-precision)"))
  (return (`self.DistanceFromPlayer`)))

(fn `PickObject`
  (`GameplayStatics.PlaySoundAtLocation` "/Game/Sounds/PickUp/S_Pickup.S_Pickup" (`self.K2_GetActorLocation`) (struct) 1.0 1.0 0.0 null null null)
  (`self.K2_DestroyActor`)
  (return))

(fn `RotateTowardsPlayer`
  (params (Object :type "SceneComponent Object Reference") (Offset :type "Rotator Structure"))
  (`SceneComponent.K2_SetWorldRotation` Object (`KismetMathLibrary.ComposeRotators` (`KismetMathLibrary.FindLookAtRotation` (`SceneComponent.K2_GetComponentLocation` Object) (`self.K2_GetActorLocation` (`GameplayStatics.GetPlayerCameraManager` 0))) Offset) false false))

(fn `UserConstructionScript`)