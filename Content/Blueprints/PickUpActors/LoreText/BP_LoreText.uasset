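; BP_LoreText is a lore note pickup that shows its text on screen when picked up.
; PickObject plays a sound, hands input from the character to itself, blends the view to itself, then creates a Widget_TextLore filled with TextNote.
; While active, BackAction removes the widget, restores character input and blends the view back.
; Paired control macros handle each input and camera handoff, with IsActive gating the exit.
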(event `InputAction|BackAction`
  (params (Key :type "Key Structure"))
  (:`Pressed`
    (if (`self.IsActive`)
      (`self.RemoveWidgetFromScreen`)
      (`self.EnablePlayerControl`
        (:`Blended`
          (set `self.IsActive` false))))))

(fn `AddWidgetToScreen`
  (bind _returnvalue (`|CreateWidget` "/Game/Blueprints/PickUpActors/LoreText/Widget_TextLore.Widget_TextLore_C" (`GameplayStatics.GetPlayerController` 0)))
  (bind _output_get (set `self.Widget` _returnvalue))
  (set `/Game/Blueprints/PickUpActors/LoreText/Widget_TextLore.LoreText` (`self.TextNote`) _output_get)
  (`UserWidget.AddToPlayerScreen` _output_get 10))

(fn `PickObject`
  (`GameplayStatics.PlaySoundAtLocation` "/Game/Sounds/PickUp/S_Pickup.S_Pickup" (`self.K2_GetActorLocation`) (struct) 1.0 1.0 0.0 null null null)
  (`self.EnableTextControl`
    (:`Blended`
      (`self.AddWidgetToScreen`)
      (set `self.IsActive` true))))

(fn `RemoveWidgetFromScreen`
  (bind _widget (`self.Widget`))
  (`/Engine/EditorBlueprintResources/StandardMacros.IsValid` _widget
    (:`Is Valid`
      (`Widget.RemoveFromParent` _widget))
    (:`Is Not Valid`
      _))
  (return))

(fn `UserConstructionScript`
  (`parent.UserConstructionScript`))