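; Ammo pickup actor that adds pistol or rifle ammo to the player's matching weapon.
; The construction script sets the pickup icon sprite from AmmoType.
; The pick-object interface event runs PickObject, which casts player 0 to BP_PlayerCharacter, calls AddAmmo on the selected weapon, then hands off to the parent PickObject.
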(event `/Game/Blueprints/PickUpActors/BPI_PickUp.BPI PickObject`
  (`self.PickObject`))

(fn `PickObject`
  (bind _asbp_player_character (cast `/Game/AdvancedLocomotionV4/Blueprints/Custom/BP_PlayerCharacter` (`GameplayStatics.GetPlayerCharacter` 0)))
  (switch `/Game/Blueprints/E_WeaponType` (`self.AmmoType`)
    (:`NewEnumerator0`
      (`/Game/Blueprints/BPC_Weapon.AddAmmo` (`/Game/AdvancedLocomotionV4/Blueprints/Custom/BP_PlayerCharacter.Pistol` _asbp_player_character) (`self.Ammo`)))
    (:`NewEnumerator1`
      (`/Game/Blueprints/BPC_Weapon.AddAmmo` (`/Game/AdvancedLocomotionV4/Blueprints/Custom/BP_PlayerCharacter.Rifle` _asbp_player_character) (`self.Ammo`))))
  (`parent.PickObject`) ; DestroyActor
)

(fn `UserConstructionScript`
  (`parent.UserConstructionScript`)
  (switch `/Game/Blueprints/E_WeaponType` (`self.AmmoType`)
    (:`NewEnumerator0`
      (`BillboardComponent.SetSprite` (`self.PickUpIcon`) "/Game/Textures/GUI/T_PistolIcon_D.T_PistolIcon_D"))
    (:`NewEnumerator1`
      (`BillboardComponent.SetSprite` (`self.PickUpIcon`) "/Game/Textures/GUI/T_RifleIcon_D.T_RifleIcon_D"))))