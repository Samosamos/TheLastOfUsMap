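; Swinging door the player opens with an input action, enabled with a prompt while inside its trigger.
; Box traces on front and back triggers find the player's side, which either shows a temporary locked message or sets the swing direction by negating the open rotation.
; Opening notifies the player character, unlocks both sides and drives a rotation timeline with sound.
; A retriggerable delay then reverses the timeline to close the door automatically.
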(event `self.InputTrigger.OnComponentBeginOverlap`
  (params (OverlappedComponent :type "PrimitiveComponent Object Reference") (OtherActor :type "Actor Object Reference") (OtherComp :type "PrimitiveComponent Object Reference") (OtherBodyIndex :type Integer) (bFromSweep :type Boolean) (SweepResult :type "HitResult Structure (by ref)"))
  ;[1 1 1] Input Trigger
  (cast `/Game/AdvancedLocomotionV4/Blueprints/Custom/BP_PlayerCharacter` OtherActor)
  (`self.EnableInput` (`GameplayStatics.GetPlayerController` 0))
  (`SceneComponent.SetVisibility` (`self.InputText`) true false)
  (`SceneComponent.SetVisibility` (`self.InputTextBack`) true false))

(event `self.InputTrigger.OnComponentEndOverlap`
  (params (OverlappedComponent :type "PrimitiveComponent Object Reference") (OtherActor :type "Actor Object Reference") (OtherComp :type "PrimitiveComponent Object Reference") (OtherBodyIndex :type Integer))
  ;[1 1 1] Input Trigger
  (cast `/Game/AdvancedLocomotionV4/Blueprints/Custom/BP_PlayerCharacter` OtherActor)
  (`self.DisableInput` (`GameplayStatics.GetPlayerController` 0))
  (`SceneComponent.SetVisibility` (`self.InputText`) false false)
  (`SceneComponent.SetVisibility` (`self.InputTextBack`) false false))

(event `StartOpenDoor`
  (bind _relativerotation (`SceneComponent.RelativeRotation` (`self.DoorMesh`)))
  ;[1 1 1] Door Side Check
  (bind _getplayer (`self.CheckPlayerInBox` (`self.FrontTrigger`)))
  (if _getplayer
    (if (`self.bIsLockedInFront?`)
      (`self.ShowLockText` true)
      (else
        (`self.SetCurrentAndTargetRotator` _relativerotation (`self.OpenedRotator`))
        (`self.OpenDoor`)))
    (else
      (bind _getplayer_2 (`self.CheckPlayerInBox` (`self.BackTrigger`)))
      (if _getplayer_2
        (if (`self.bIsLockedInBack?`)
          (`self.ShowLockText` false true)
          (else
            (`self.SetCurrentAndTargetRotator` _relativerotation (`KismetMathLibrary.NegateRotator` (`self.OpenedRotator`)))
            (`self.OpenDoor`)))))))

(event `ShowLockText`
  (params (ShowFront :type Boolean) (ShowBack :type Boolean))
  ;[1 1 1] Locked Text Visibility
  (`SceneComponent.SetVisibility` (`self.LockTextFront`) ShowFront false)
  (`SceneComponent.SetVisibility` (`self.LockTextBack`) ShowBack false)
  (`KismetSystemLibrary.RetriggerableDelay` 5.0)
  (`SceneComponent.SetVisibility` (`self.LockTextFront`) false false)
  (`SceneComponent.SetVisibility` (`self.LockTextBack`) false false))

(event `self.ReceiveBeginPlay`
  (`SceneComponent.SetVisibility` (`self.InputText`) false false)
  (`SceneComponent.SetVisibility` (`self.InputTextBack`) false false))

(event `InputAction|OpenDoorAction`
  (params (Key :type "Key Structure"))
  ;[1 1 1] Input event
  (:`Pressed`
    (if (not (`self.bIsOpen?`))
      (`self.StartOpenDoor`))))

(event `OpenDoor`
  ;[1 1 1] Open/Close Door
  (bind _asbp_player_character (cast `/Game/AdvancedLocomotionV4/Blueprints/Custom/BP_PlayerCharacter` (`GameplayStatics.GetPlayerPawn` 0)))
  (`/Game/AdvancedLocomotionV4/Blueprints/Custom/BP_PlayerCharacter.OpenDoorEvent` _asbp_player_character)
  (set `self.bIsOpen?` true)
  (`GameplayStatics.PlaySoundAtLocation` "/Game/BlockingStarterPack/Sounds/SimpleDoor_StartOpening_Cue.SimpleDoor_StartOpening_Cue" (`self.K2_GetActorLocation`) (struct) 1.0 1.0 0.0 null null null)
  (`self.UnlockDoor` true)
  (bind (_direction _opentrack) (`Timeline|DoorOpening` :!via `PlayFromStart` :!label _label)
    (:`Update`
      (bind _returnvalue (`KismetMathLibrary.RLerp` (`self.CurrentRotator`) (`self.TargetRotator`) _opentrack))
      (`SceneComponent.K2_SetRelativeRotation` (`self.DoorMesh`) _returnvalue false false))
    (:`Finished`
      (`self.SetCurrentAndTargetRotator` (`self.ClosedRotator`) _returnvalue)
      (if (`self.bIsOpen?`)
        (`KismetSystemLibrary.RetriggerableDelay` 5.0)
        (set `self.bIsOpen?` false)
        (goto _label :!via `ReverseFromEnd`)
        (else
          (`GameplayStatics.PlaySoundAtLocation` "/Game/BlockingStarterPack/Sounds/SimpleDoor_Closing_Cue.SimpleDoor_Closing_Cue" (`self.K2_GetActorLocation`) (struct) 1.0 1.0 0.0 null null null))))))

(fn `CheckPlayerInBox`
  (params (BoxCollision :type "BoxComponent Object Reference"))
  (returns (GetPlayer :type Boolean))
  (bind _returnvalue (`SceneComponent.K2_GetComponentLocation` BoxCollision))
  (bind _outhits (`KismetSystemLibrary.BoxTraceMultiForObjects` _returnvalue _returnvalue (`BoxComponent.GetScaledBoxExtent` BoxCollision) (`self.K2_GetActorRotation`) (`|MakeArray` "ObjectTypeQuery3" :!type "EObjectTypeQuery Enum")))
  (for _array_element _outhits
    (cast `/Game/AdvancedLocomotionV4/Blueprints/Custom/BP_PlayerCharacter` (`.HitActor` (`GameplayStatics.BreakHitResult` _array_element)))
    (return true))
  (return false))

(fn `SetCurrentAndTargetRotator`
  (params (Current :type "Rotator Structure") (Target :type "Rotator Structure"))
  (set `self.CurrentRotator` Current)
  (set `self.TargetRotator` Target)
  (return))

(fn `UnlockDoor`
  (params (UnlockFrontLock :type Boolean :default true) (UnlockBackLock :type Boolean :default true))
  (set `self.bIsLockedInFront?` (not UnlockFrontLock))
  (set `self.bIsLockedInBack?` (not UnlockBackLock))
  (return))

(fn `UserConstructionScript`)