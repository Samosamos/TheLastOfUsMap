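; Weapon component that tracks loaded and reserve ammo and handles shooting and reloading for its owning actor.
; Shoot checks ammo and busy state, spends a round, sets the shooting flag, plays a 2D shot sound and has a BP_PlayerCharacter owner report stance-independent noise.
; Reload takes new ammo counts from a ReloadAmmo helper; AddAmmo feeds the reserve, and wrapper functions expose the shoot and reload checks.
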(fn `AddAmmo`
  (params (AmmoToAdd :type Integer))
  (set `self.AmmoInStock` (+ AmmoToAdd (`self.AmmoInStock`)))
  (return))

(fn `CanReloadWeapon`
  (returns (CanReload :type Boolean))
  (return (`self.CanReload`)))

(fn `CanShootWithWeapon`
  (returns (CanShoot :type Boolean))
  (return (`self.CanShoot`)))

(fn `Reload`
  (bind (_newloadedammo _newammoinstock) (`/Game/Blueprints/Libraries/BPF_ReloadAmmo.ReloadAmmo` (`self.MaxLoadedAmmo`) (`self.LoadedAmmo`) (`self.AmmoInStock`)))
  (set `self.LoadedAmmo` _newloadedammo)
  (set `self.AmmoInStock` _newammoinstock)
  (return))

(fn `Shoot`
  (if (`self.CanShoot`)
    (`/Engine/EditorBlueprintResources/StandardMacros.DecrementInt` (`self.LoadedAmmo`)
      (:`  `
        (set `self.bIsShooting?` true)
        (`GameplayStatics.PlaySound2D` (`self.WeaponShotSound`) 1.0 1.0 0.0 null null)
        (bind _asbp_player_character (cast `/Game/AdvancedLocomotionV4/Blueprints/Custom/BP_PlayerCharacter` (`self.GetOwner`))
          (:`then`
            (`/Game/AdvancedLocomotionV4/Blueprints/Custom/BP_PlayerCharacter.ReportNoise` _asbp_player_character true 1000.0))
          (:`CastFailed`
            _))
        (return)))))