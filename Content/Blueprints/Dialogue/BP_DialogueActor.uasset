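; BP_DialogueActor is a dialogue actor that plays an array of dialogue sounds in sequence through its Audio component.
; PlayDialogue sets the component's sound to the entry at DialogueIndex, fetched by GetDialogue, and plays it.
; BeginPlay binds the audio-finished event to NextDialogue, which increments the index and plays again while entries remain.
; BeginPlay only binds the event and does not call PlayDialogue.
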(event `self.ReceiveBeginPlay`
  (add `AudioComponent.OnAudioFinished` (`self.Audio`) (delegate `NextDialogue`)))

(event `NextDialogue`
  ;[1 1 1] NextDialogue
  (bind _result (`/Engine/EditorBlueprintResources/StandardMacros.IncrementInt` (`self.DialogueIndex`))
    (:`  `
      (if (< _result (`KismetArrayLibrary.Array_Length` (`self.DialogueSound`)))
        (`self.PlayDialogue`)))))

(event `PlayDialogue`
  (bind _audio (`self.Audio`))
  ;[1 1 1] Play Dialogue
  (`AudioComponent.SetSound` _audio (`self.GetDialogue` (`self.DialogueIndex`)))
  (`AudioComponent.Play` _audio 0.0))

(fn `GetDialogue`
  (params (Index :type Integer))
  (returns (SoundCue :type "SoundBase Object Reference"))
  (return (`|GetArrayItem` (`self.DialogueSound`) Index)))

(fn `UserConstructionScript`)